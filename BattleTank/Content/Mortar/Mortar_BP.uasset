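; Mortar actor that sets up tank-style aiming and is destroyed by cannon projectiles.
; On BeginPlay it passes its TankBarrel and TankTurret to the TankAiming component.
; An overlap with a CannonProjectile_BP prints a "Boink!" message, spawns an explosion emitter at the mortar's location and destroys the mortar outright, with no health or damage step.
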(event EventBeginPlay
  (Class|TankAimingComponent|Initialise (Variables|Default|GetTankAiming) (Variables|Default|GetTankBarrel) (Variables|Default|GetTankTurret)))

(event Collision|EventActorBeginOverlap
  (params (OtherActor :type Actor%20Object%20Reference))
  (if (== OtherActor "/Game/Tank/CannonProjectile_BP.CannonProjectile_BP_C")
    (Development|PrintString "Boink!")
    (Effects|SpawnEmitteratLocation "/Game/Particle/P_Explosion.P_Explosion" (Transformation|GetActorLocation))
    (Actor|DestroyActor)))

(fn ConstructionScript)