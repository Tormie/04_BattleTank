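; Tank Blueprint that serves both player and AI tanks, with a free-look aiming camera.
; On BeginPlay it registers the Barrel through SetBarrelReference and picks the hull material by whether a TankAIController possesses it.
; Aim axis inputs rotate the azimuth gimbal and spring arm, scaled by delta time, leaving turret and barrel untouched.
; Older direct turret rotation and clamped barrel elevation logic remains disconnected.
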(event EventBeginPlay
  (Class|Tank|SetBarrelReference (Variables|Default|GetBarrel))
  ;[1 1 1] Set Material based on type of controller (AI or player)
  (bind _returnvalue (AI|GetAIController self))
  (if (Utilities|ClassIsChildOf (Utilities|GetClass _returnvalue) "/Script/BattleTank.TankAIController")
    (Rendering|Material|SetMaterial (Variables|Default|GetTank) 0 "/Game/Tank/M_Metal_Tank_AI.M_Metal_Tank_AI")
    (else
      (Rendering|Material|SetMaterial (Variables|Default|GetTank) 0 "/Game/Tank/M_Metal_Tank.M_Metal_Tank"))))

(event EventActorBeginOverlap
  (params (OtherActor :type Actor%20Object%20Reference)))

(event EventTick
  (params (DeltaSeconds :type Float%20%28single-precision%29)))

(event Input|AxisEvents|InputAxisAimElevation
  (params (AxisValue :type Float%20%28single-precision%29))
  ;[1 1 1] Basic rotation and elevation
  (Transformation|AddLocalRotation (Variables|Default|GetSpringArm) (Math|Rotator|MakeRotator 0.0 (* AxisValue (Utilities|Time|GetWorldDeltaSeconds) 1e+02) 0.0) false false))

(event Input|AxisEvents|InputAxisAimAzimuth
  (params (AxisValue :type Float%20%28single-precision%29))
  ;[1 1 1] Basic rotation and elevation
  (Transformation|AddLocalRotation (Variables|Default|GetAzimuth%20Gimbal) (Math|Rotator|MakeRotator 0.0 0.0 (* AxisValue (Utilities|Time|GetWorldDeltaSeconds) 1e+02)) false false))

(fn ConstructionScript)